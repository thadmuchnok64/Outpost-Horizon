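; Grabbable lever component that acts as a spring-return switch with both on/off and analog output.
; While held, it aims its original parent by the clamped look-at pitch between them, applied as roll.
; That angle feeds a normalized RawLeverValue and flips SwitchState near either limit, leaving a dead band between.
; ResetLeverPosition waits briefly, then if released eases the parent back to its original transform and clears SwitchState.
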(event `self.ReceiveTick`
  (params (DeltaSeconds :type "Float (single-precision)"))
  (bind _returnvalue (`KismetMathLibrary.ClampAngle` (.pitch (`KismetMathLibrary.FindLookAtRotation` (`self.K2_GetComponentLocation`) (`self.K2_GetComponentLocation` (`self.OriginalParent`)))) (`self.MinLeverPush`) (`self.MaxLeverPush`)))
  (set `self.SnapCooldown` (- (`self.SnapCooldown`) 0.0))
  (if (`self.bIsHeld`)
    (`|ExecutionSequence`
      (:`then_0`
        (goto _label :!via `Stop`))
      (:`then_1`
        ;[1 1 1] Check if switch is flipped and clamp switch rotation
        (set `self.RawLeverValue` (`KismetMathLibrary.MapRangeClamped` _returnvalue (`self.MinLeverPush`) (`self.MaxLeverPush`) -1.0 1.0))
        (if (< _returnvalue (+ (`self.MinLeverPush`) 15.0))
          (set `self.SwitchState` false)
          (elif (> _returnvalue (+ (`self.MaxLeverPush`) -15.0))
            (set `self.SwitchState` true)))
        (`self.K2_SetRelativeRotation` (`self.OriginalParent`) (`KismetMathLibrary.MakeRotator` _returnvalue) false false)))))

(event `ResetLeverPosition`
  ;[1 1 1] Lever Reset
  (`KismetSystemLibrary.Delay` 0.3)
  (if (not (`self.bIsHeld`))
    (`KismetSystemLibrary.MoveComponentTo` (`self.OriginalParent`) (.location (`self.ParentOriginalTransform`)) (.rotation (`self.ParentOriginalTransform`)) false true 0.1 :!label _label)
    (set `self.SwitchState` false)))
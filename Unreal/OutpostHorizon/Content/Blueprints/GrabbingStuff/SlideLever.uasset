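; SlideLever is a grabbable lever component that slides along a single axis and outputs a normalized lever value.
; ManageLever projects the component's world location onto the right-vector line through OriginalParent and moves OriginalParent to that point.
; It then clamps the parent's relative Y between the push limits and maps that position to RawLeverValue from -1 to 1.
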(fn `Manage Lever`
  (bind _originalparent (`self.OriginalParent`))
  (bind _originalparent_2 (`self.OriginalParent`))
  (bind _returnvalue (`KismetMathLibrary.FClamp` (.y (`SceneComponent.RelativeLocation` _originalparent_2)) (`self.MinLeverPush`) (`self.MaxLeverPush`)))
  ;[1 1 1] PushLever
  (`self.K2_SetWorldLocation` _originalparent_2 (`KismetMathLibrary.FindClosestPointOnLine` (`self.K2_GetComponentLocation`) (`self.K2_GetComponentLocation` _originalparent) (`self.GetRightVector` _originalparent)) false false)
  (`self.K2_SetRelativeLocation` (`self.OriginalParent`) (`KismetMathLibrary.MakeVector` (.x (`SceneComponent.RelativeLocation` _originalparent_2)) _returnvalue (.z (`SceneComponent.RelativeLocation` _originalparent_2))) false true)
  (set `self.RawLeverValue` (`KismetMathLibrary.MapRangeClamped` _returnvalue (`self.MinLeverPush`) (`self.MaxLeverPush`) -1.0 1.0)))
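; FlipLever is a grabbable-style lever switch that outputs an on/off state and an analog value.
; ManageLever takes the look-at pitch from its own location to OriginalParent, clamps it to the push limits and applies it as the parent's relative roll.
; The same angle maps to RawLeverValue from -1 to 1.
; SwitchState flips only near either limit, holding in between as hysteresis.
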(fn `Manage Lever`
  (bind _returnvalue (`KismetMathLibrary.ClampAngle` (.pitch (`KismetMathLibrary.FindLookAtRotation` (`self.K2_GetComponentLocation`) (`self.K2_GetComponentLocation` (`self.OriginalParent`)))) (`self.MinLeverPush`) (`self.MaxLeverPush`)))
  ;[1 1 1] Check if switch is flipped and clamp switch rotation
  (set `self.RawLeverValue` (`KismetMathLibrary.MapRangeClamped` _returnvalue (`self.MinLeverPush`) (`self.MaxLeverPush`) -1.0 1.0))
  (if (< _returnvalue (+ (`self.MinLeverPush`) 15.0))
    (set `self.SwitchState` false)
    (elif (> _returnvalue (+ (`self.MaxLeverPush`) -15.0))
      (set `self.SwitchState` true)))
  (`self.K2_SetRelativeRotation` (`self.OriginalParent`) (`KismetMathLibrary.MakeRotator` _returnvalue) false false))
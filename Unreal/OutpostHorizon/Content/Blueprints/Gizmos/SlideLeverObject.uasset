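; SlideLeverObject is a slide lever gizmo actor that plays a cranking sound as the lever moves.
; On BeginPlay it hands its Pivot component to the SlideLever as the custom pivot.
; Each tick it rounds the raw lever value to tenths and, when that step changes, plays LeverCrank at the pivot with a pitch derived from the step.
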(event `self.ReceiveBeginPlay`
  (set `/Game/Blueprints/GrabbingStuff/GrabComponent.CustomPivot` (`self.Pivot`) (`self.SlideLever`)))

(event `self.ReceiveTick`
  (params (DeltaSeconds :type "Float (single-precision)"))
  (bind _returnvalue (`KismetMathLibrary.Round` (* (`/Game/Blueprints/GrabbingStuff/Lever.RawLeverValue` (`self.SlideLever`)) 10.0)))
  (if (!= (`self.LeverRound`) _returnvalue)
    (bind _output_get (set `self.LeverRound` _returnvalue))
    (`GameplayStatics.PlaySoundAtLocation` "/Game/Sounds/Sound_Effects/LeverCrank.LeverCrank" (`SceneComponent.K2_GetComponentLocation` (`self.Pivot`)) (struct) 1.0 (`KismetMathLibrary.Conv_IntToDouble` (+ (/ _output_get 4) 1)) 0.0 null null null null)))

(fn `UserConstructionScript`)
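; Door control gizmo with a child-actor button that calls OnPicked on its door once the lock is released.
; On BeginPlay it binds Unlock to the DoorWall's unlock event, which clears the Locked flag and switches a CRTV material to Unlocked.
; Tick polls the button's pressed state, and a DoOnce with no reset limits the door trigger to a single firing.
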(event `self.ReceiveBeginPlay`
  (add `/Game/Blueprints/BuildingBlocks/WallDoor.UnlockDoor` (`self.DoorWall`) (delegate `Unlock`)))

(event `Unlock`
  (`PrimitiveComponent.SetMaterial` (`self.CRTV`) 1 "/Game/Materials/CRTV/Power/Unlocked.Unlocked")
  (set `self.Locked` false))

(event `self.ReceiveTick`
  (params (DeltaSeconds :type "Float (single-precision)"))
  (bind _asbutton (cast `/Game/Blueprints/Gizmos/Button` (`ChildActorComponent.ChildActor` (`self.Button`))))
  (if (and (`/Game/Blueprints/Gizmos/Button.IsBeingPressed` _asbutton) (not (`self.Locked`)))
    (`/Engine/EditorBlueprintResources/StandardMacros.DoOnce` false
      (:`Completed`
        (`/Game/Blueprints/Gizmos/Door.OnPicked` (`self.Door`))))))

(fn `UserConstructionScript`)
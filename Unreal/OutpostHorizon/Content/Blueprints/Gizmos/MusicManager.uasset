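; MusicManager is an actor that controls background music through a single audio component.
; Request functions for the fuel rod, crane game and Noire songs each stop the current sound and play their track, guarded by flags so each plays only once.
; RequestAmbiance starts a passed-in song only when nothing is playing, and StopSong fades the audio out.
; All logic is in these callable functions, with empty event and construction graphs.
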(fn `Request Ambiance`
  (params (Song :type "SoundWave Object Reference"))
  (bind _audio (`self.Audio`))
  (if (not (`AudioComponent.IsPlaying` _audio))
    (`AudioComponent.Stop` _audio)
    (`AudioComponent.SetSound` _audio Song)
    (`AudioComponent.Play` _audio 0.0)))

(fn `Request Crane Game Song`
  (bind _audio (`self.Audio`))
  (if (not (`self.Crane Played`))
    (set `self.Crane Played` true)
    (`AudioComponent.Stop` _audio)
    (`AudioComponent.SetSound` _audio "/Game/Sounds/Music/cranegame.cranegame")
    (`AudioComponent.Play` _audio 0.0)))

(fn `Request Fuel Rod Song`
  (bind _audio (`self.Audio`))
  (if (not (`self.Fuel Rod Played`))
    (set `self.Fuel Rod Played` true)
    (`AudioComponent.Stop` _audio)
    (`AudioComponent.SetSound` _audio "/Game/Sounds/Music/Rods.Rods")
    (`AudioComponent.Play` _audio 0.0)))

(fn `Request Noire Song`
  (bind _audio (`self.Audio`))
  (if (not (`self.NoirePlayed`))
    (set `self.NoirePlayed` true)
    (`AudioComponent.Stop` _audio)
    (`AudioComponent.SetSound` _audio "/Game/Sounds/Music/MrNoire.MrNoire")
    (`AudioComponent.Play` _audio 0.0)))

(fn `StopSong`
  (`AudioComponent.FadeOut` (`self.Audio`) 2.0 0.0 "Linear"))

(fn `UserConstructionScript`)
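; Button gizmo that starts the credits sequence on a CRT TV, using the title screen parameter collection.
; Tick polls the child Button actor and, on the first press, briefly flashes static on the TV, switches to the ending material and plays the credits sound.
; After a short delay, Tick begins driving a clamped, timer-based scroll parameter in that Material Parameter Collection.
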(event `self.ReceiveTick`
  (params (DeltaSeconds :type "Float (single-precision)"))
  (`|ExecutionSequence`
    (:`then_0`
      (if (`self.RollingCredits`)
        (bind _output_get (set `self.Timer` (+ (`self.Timer`) DeltaSeconds)))
        (`KismetMaterialLibrary.SetScalarParameterValue` "/Game/Materials/TitleScreenParams.TitleScreenParams" "CreditsScroll" (`KismetMathLibrary.FClamp` (/ _output_get 75.0) 0.0 0.53))))
    (:`then_1`
      (bind _asbutton (cast `/Game/Blueprints/Gizmos/Button` (`ChildActorComponent.ChildActor` (`self.Button`))))
      (if (`/Game/Blueprints/Gizmos/Button.IsBeingPressed` _asbutton)
        (`/Engine/EditorBlueprintResources/StandardMacros.DoOnce` false
          (:`Completed`
            (`PrimitiveComponent.SetMaterial` (`self.CRTV`) 1 "/Game/Materials/CRTV/Power/Static.Static")
            (`KismetSystemLibrary.Delay` 0.3)
            (`PrimitiveComponent.SetMaterial` (`self.CRTV`) 1 "/Game/Materials/CRTV/Power/EndingTime.EndingTime")
            (`GameplayStatics.PlaySound2D` "/Game/Sounds/Music/Credits.Credits" 1.0 1.0 0.0 null null)
            (`KismetSystemLibrary.Delay` 2.0)
            (set `self.RollingCredits` true)))))))

(fn `UserConstructionScript`)
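; Radio actor that plays one of four noir character voice clips over a music track.
; Each NoirGuy event calls StartNoir, then swaps its clip into the Dialogue audio component and plays it from the start.
; StartNoir restarts the Music component and stops it after a fixed Delay, which a repeat call does not reset while pending.
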(event `self.ReceiveBeginPlay`)

(event `StartNoir`
  (bind _music (`self.Music`))
  (`AudioComponent.Stop` _music)
  (`AudioComponent.Play` _music 0.0)
  (`KismetSystemLibrary.Delay` 30.0)
  (`AudioComponent.Stop` _music))

(event `NoirGuy1`
  (bind _dialogue (`self.Dialogue`))
  (`self.StartNoir`)
  (`AudioComponent.Stop` _dialogue)
  (`AudioComponent.SetSound` _dialogue "/Game/Sounds/NoirVoice/NoirGuy1.NoirGuy1")
  (`AudioComponent.Play` _dialogue 0.0))

(event `NoirGuy2`
  (bind _dialogue (`self.Dialogue`))
  (`self.StartNoir`)
  (`AudioComponent.Stop` _dialogue)
  (`AudioComponent.SetSound` _dialogue "/Game/Sounds/NoirVoice/NoirGuy2.NoirGuy2")
  (`AudioComponent.Play` _dialogue 0.0))

(event `NoirGuy3`
  (bind _dialogue (`self.Dialogue`))
  (`self.StartNoir`)
  (`AudioComponent.Stop` _dialogue)
  (`AudioComponent.SetSound` _dialogue "/Game/Sounds/NoirVoice/NoirGuy3.NoirGuy3")
  (`AudioComponent.Play` _dialogue 0.0))

(event `NoirGuy4`
  (bind _dialogue (`self.Dialogue`))
  (`self.StartNoir`)
  (`AudioComponent.Stop` _dialogue)
  (`AudioComponent.SetSound` _dialogue "/Game/Sounds/NoirVoice/NoirGuy4.NoirGuy4")
  (`AudioComponent.Play` _dialogue 0.0))

(fn `UserConstructionScript`)
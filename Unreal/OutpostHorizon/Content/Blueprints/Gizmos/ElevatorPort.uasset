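; Elevator door gizmo that opens and closes its gate according to the DoorOpen flag.
; Tick moves a clamped Timer up or down at Speed and scrubs the ElevatorGate animation through its start time offset instead of playing it.
; On opening, a DoOnce plays the open sound and disables the blocking Box's collision; closing resets it and restores collision.
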(event `self.ReceiveTick`
  (params (DeltaSeconds :type "Float (single-precision)"))
  (bind _timer (`self.Timer`))
  (bind _returnvalue (* DeltaSeconds (`self.Speed`)))
  (if (`self.DoorOpen`)
    (`|ExecutionSequence`
      (:`then_0`
        (`/Engine/EditorBlueprintResources/StandardMacros.DoOnce` false :!label _label
          (:`Completed`
            (`GameplayStatics.PlaySoundAtLocation` "/Game/Sounds/Sound_Effects/ElevatorOpen.ElevatorOpen" (`self.K2_GetActorLocation`) (struct) 1.0 1.0 0.0 "/Game/Sounds/Sound_Effects/Attenuation/SmallGizmo.SmallGizmo" null null null)
            (`PrimitiveComponent.SetCollisionEnabled` (`self.Box`) "NoCollision"))))
      (:`then_1`
        (set `self.Timer` (+ _returnvalue _timer))
        (bind _output_get (set `self.Timer` (`KismetMathLibrary.FClamp` _timer) :!label _label_2))
        (`GeometryCacheComponent.SetStartTimeOffset` (`self.Elevator_Gate`) (`KismetMathLibrary.Lerp` 0.0 5.0 _output_get))))
    (else
      (`|ExecutionSequence`
        (:`then_0`
          (goto _label :!via `Reset`))
        (:`then_1`
          (`PrimitiveComponent.SetCollisionEnabled` (`self.Box`) "QueryAndPhysics")
          (set `self.Timer` (- _timer _returnvalue))
          (goto _label_2))))))

(fn `UserConstructionScript`)
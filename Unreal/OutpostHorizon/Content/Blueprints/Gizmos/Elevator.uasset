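; Elevator gizmo with sliding double doors, operated by a child-actor Button that is polled each Tick.
; A DoOnce gate turns each press into one toggle, opening or closing the doors with eased component moves and sounds, each direction stopping the other.
; Closing also starts a slow move of the root to the height of the ElevatorPort nearest world origin, with a fixed target rotation, marked as temporary placement.
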(event `CloseDoors`
  (`|ExecutionSequence`
    (:`then_0`
      (goto _label_3 :!via `Stop`))
    (:`then_1`
      (goto _label_4 :!via `Stop`))
    (:`then_2`
      (`KismetSystemLibrary.MoveComponentTo` (`self.Elevator_Door_Left`) (* (`self.ElevatorDoorRoot`) (-1.0 1.0 1.0)) (struct) true true 1.0 :!label _label)
      (`GameplayStatics.PlaySoundAtLocation` "/Game/Sounds/Sound_Effects/Door/DoorCloseElevator.DoorCloseElevator" (`SceneComponent.K2_GetComponentLocation` (`self.Doors`)) (struct) 1.0 1.0 0.0 null null null null))
    (:`then_3`
      (`KismetSystemLibrary.MoveComponentTo` (`self.Elevator_Door_Right`) (`self.ElevatorDoorRoot`) (struct) true true 1.0 :!label _label_2))))

(event `OpenDoors`
  (`|ExecutionSequence`
    (:`then_0`
      (goto _label :!via `Stop`))
    (:`then_1`
      (goto _label_2 :!via `Stop`))
    (:`then_2`
      (`KismetSystemLibrary.MoveComponentTo` (`self.Elevator_Door_Left`) (`KismetMathLibrary.MakeVector` -63.0 (.y (`self.ElevatorDoorRoot`)) (.z (`self.ElevatorDoorRoot`))) (struct) true true 1.0 :!label _label_3))
    (:`then_3`
      (`GameplayStatics.PlaySoundAtLocation` "/Game/Sounds/Sound_Effects/Door/DoorOpenElevator.DoorOpenElevator" (`SceneComponent.K2_GetComponentLocation` (`self.Doors`)) (struct) 1.0 1.0 0.0 null null null null)
      (`KismetSystemLibrary.MoveComponentTo` (`self.Elevator_Door_Right`) (`KismetMathLibrary.MakeVector` 63.0 (.y (`self.ElevatorDoorRoot`)) (.z (`self.ElevatorDoorRoot`))) (struct) true true 1.0 :!label _label_4))))

(event `self.ReceiveBeginPlay`
  (set `self.ElevatorDoorRoot` (`SceneComponent.RelativeLocation` (`self.Elevator_Door_Right`))))

(event `self.ReceiveTick`
  (params (DeltaSeconds :type "Float (single-precision)"))
  (bind (_returnvalue_x _returnvalue_y) (`KismetMathLibrary.BreakVector` (`self.K2_GetActorLocation`)))
  (bind _asbutton (cast `/Game/Blueprints/Gizmos/Button` (`ChildActorComponent.ChildActor` (`self.Button`))))
  (if (`/Game/Blueprints/Gizmos/Button.IsBeingPressed` _asbutton)
    (`/Engine/EditorBlueprintResources/StandardMacros.DoOnce` false :!label _label_5
      (:`Completed`
        (bind _output_get (set `self.Open` (not (`self.Open`))))
        (if _output_get
          (`self.OpenDoors`)
          (else
            (`|ExecutionSequence`
              (:`then_0`
                (`self.CloseDoors`))
              (:`then_1`
                ;[1 1 1] Move this later
                (bind _outactors (`GameplayStatics.GetAllActorsOfClass` "/Game/Blueprints/Gizmos/ElevatorPort.ElevatorPort_C"))
                (bind (_returnvalue_x_2 _returnvalue_y_2 _returnvalue_z) (`KismetMathLibrary.BreakVector` (`self.K2_GetActorLocation` (`.ReturnValue` (`GameplayStatics.FindNearestActor` (0.0 0.0 0.0) _outactors)))))
                (`KismetSystemLibrary.MoveComponentTo` (`self.DefaultSceneRoot`) (`KismetMathLibrary.MakeVector` _returnvalue_x _returnvalue_y _returnvalue_z) (struct :`Yaw` 180.0) true true 15.0)))))))
    (else
      (goto _label_5 :!via `Reset`))))

(fn `UserConstructionScript`)
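; Gizmo that mirrors the level layout to a connected Unity user through TCPClient.
; When that user is online, it gathers transforms of tagged static meshes and gameplay actors such as doors, elevators and cranes.
; It resets the remote map, then sends each type by item code in delayed, recursive batches.
; Remote elevator triggers move stored elevators by index; the bound door-open handler is empty, its unlock logic disconnected.
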(event `self.ReceiveBeginPlay`
  (bind _returnvalue (`GameplayStatics.GetActorOfClass` "/Game/NetworkStuff/TCPClient.TCPClient_C"))
  (if (`/Game/NetworkStuff/TCPClient.isUnityUserOnline` _returnvalue)
    (`self.SendMapInfo`))
  (`|ExecutionSequence`
    (:`then_0`
      (add `/Game/NetworkStuff/TCPClient.UnityUserOnline` _returnvalue (delegate `SendMapInfo`)))
    (:`then_1`
      (add `/Game/NetworkStuff/TCPClient.OpenDoorRemotely` _returnvalue (delegate `OpenDoor`)))
    (:`then_2`
      (add `/Game/NetworkStuff/TCPClient.TriggerElevatorRemotely` _returnvalue (delegate `TriggerElevator`)))))

(event `SendMapInfo`
  ;[1 1 1] We need to set this so this happens when the unity user connects. not beginplay
  (`KismetSystemLibrary.Delay` 5.0)
  (set `self.WallArray` (`|MakeArray`))
  (set `self.FloorArray` (`|MakeArray`))
  (bind _outactors (`GameplayStatics.GetAllActorsOfClass` "/Script/Engine.StaticMeshActor"))
  (for _array_element _outactors
    (if (`self.ActorHasTag` _array_element "UnityMap")
      (`|ExecutionSequence`
        (:`then_0`
          (if (`self.ActorHasTag` _array_element "Floor")
            (bind _array (`|MakeArray` (`SceneComponent.GetRelativeTransform` (`StaticMeshActor.StaticMeshComponent` _array_element))))
            (`KismetArrayLibrary.Array_Append` (`self.FloorArray`) _array)))
        (:`then_1`
          (if (`self.ActorHasTag` _array_element "Wall")
            (`KismetArrayLibrary.Array_Append` (`self.WallArray`) _array)))
        (:`then_2`
          (if (`self.ActorHasTag` _array_element "ControlRoom")
            (`KismetArrayLibrary.Array_Append` (`self.ControlRoom`) _array)))
        (:`then_3`
          (if (`self.ActorHasTag` _array_element "Crate")
            (`KismetArrayLibrary.Array_Append` (`self.SmallCrates`) _array)))
        (:`then_4`
          (if (`self.ActorHasTag` _array_element "CraneControl")
            (`KismetArrayLibrary.Array_Append` (`self.CraneControl`) _array))))))
  (`|ExecutionSequence`
    (:`then_0`
      (bind _outactors_2 (`GameplayStatics.GetAllActorsOfClass` "/Game/Blueprints/Gizmos/Elevator.Elevator_C"))
      (for _array_element_2 _outactors_2
        (`KismetArrayLibrary.Array_Append` (`self.ElevatorArray`) (`|MakeArray` (`self.GetTransform` _array_element_2)))
        (`KismetArrayLibrary.Array_Append` (`self.ElevatorReference`) (`|MakeArray` _array_element_2))))
    (:`then_1`
      (bind _outactors_3 (`GameplayStatics.GetAllActorsOfClass` "/Game/Blueprints/Gizmos/ElevatorPort.ElevatorPort_C"))
      (for _array_element_3 _outactors_3
        (`KismetArrayLibrary.Array_Append` (`self.ElevatorPortArray`) (`|MakeArray` (`self.GetTransform` _array_element_3)))))
    (:`then_2`
      (bind _outactors_4 (`GameplayStatics.GetAllActorsOfClass` "/Game/Blueprints/BuildingBlocks/WallDoor.WallDoor_C"))
      (for (_array_element_4 _array_index) _outactors_4
        (set `/Game/Blueprints/BuildingBlocks/WallDoor.DoorCode` _array_index _array_element_4)
        (`KismetArrayLibrary.Array_Append` (`self.DoorArray`) (`|MakeArray` (`self.GetTransform` _array_element_4)))))
    (:`then_3`
      (bind _outactors_5 (`GameplayStatics.GetAllActorsOfClass` "/Game/Blueprints/EngineRoom/Engine_Blueprint.Engine_Blueprint_C"))
      (for _array_element_5 _outactors_5
        (`KismetArrayLibrary.Array_Append` (`self.Engine`) (`|MakeArray` (`self.GetTransform` _array_element_5)))))
    (:`then_4`
      (bind _outactors_6 (`GameplayStatics.GetAllActorsOfClass` "/Game/Blueprints/CraneRoom/Crane_New.Crane_New_C"))
      (for _array_element_6 _outactors_6
        (`KismetArrayLibrary.Array_Append` (`self.Crane`) (`|MakeArray` (`self.GetTransform` _array_element_6)))))
    (:`then_5`
      (bind _returnvalue (`GameplayStatics.GetActorOfClass` "/Game/NetworkStuff/TCPClient.TCPClient_C"))
      (`/Game/NetworkStuff/TCPClient.SendMessageToServer` _returnvalue "ResetWorldMap" 2)
      (`KismetSystemLibrary.Delay` 0.1)
      (`self.LoopMessage` (`self.FloorArray`) 1)
      (`KismetSystemLibrary.Delay` 1.0)
      (`self.LoopMessage` (`self.WallArray`) 2)
      (`KismetSystemLibrary.Delay` 1.0)
      (`self.LoopMessage` (`self.DoorArray`) 3)
      (`KismetSystemLibrary.Delay` 0.5)
      (`self.LoopMessage` (`self.ElevatorArray`) 4)
      (`KismetSystemLibrary.Delay` 0.5)
      (`self.LoopMessage` (`self.ElevatorPortArray`) 5)
      (`KismetSystemLibrary.Delay` 0.2)
      (`self.LoopMessage` (`self.ControlRoom`) 6)
      (`KismetSystemLibrary.Delay` 0.2)
      (`self.LoopMessage` (`self.SmallCrates`) 7)
      (`KismetSystemLibrary.Delay` 0.2)
      (`self.LoopMessage` (`self.Engine`) 8)
      (`KismetSystemLibrary.Delay` 0.2)
      (`self.LoopMessage` (`self.Crane`) 9)
      (`KismetSystemLibrary.Delay` 0.2)
      (`self.LoopMessage` (`self.CraneControl`) 10))))

(event `OpenDoor`
  (params (DoorCode :type Integer))
  ;[1 1 1] Remote Door Opening
)

(event `TriggerElevator`
  (params (Code :type Integer))
  ;[1 1 1] Move Elevator with Phone
  (`/Game/Blueprints/Gizmos/Elevator.MoveElevator` (`|GetArrayItem` (`self.ElevatorReference`) Code)))

(event `LoopMessage`
  (params (Transforms :type "Array of Transform Structure") (ItemCode :type Integer))
  (set `self.Batch` (`|MakeArray`))
  (for _ (range 21)
    (if (> (`KismetArrayLibrary.Array_Length` Transforms) 0)
      (`KismetArrayLibrary.Array_Append` (`self.Batch`) (`|MakeArray` (`|GetArrayItem` Transforms)))
      (`KismetArrayLibrary.Array_Remove` Transforms)
      (else
        (break))))
  (bind _returnvalue (`GameplayStatics.GetActorOfClass` "/Game/NetworkStuff/TCPClient.TCPClient_C"))
  (`/Game/NetworkStuff/TCPClient.SendMapInformationToServer` _returnvalue (`self.Batch`) ItemCode)
  (if (> (`KismetArrayLibrary.Array_Length` Transforms) 0)
    (`KismetSystemLibrary.Delay` 0.1)
    (`self.LoopMessage` Transforms ItemCode)))

(fn `UserConstructionScript`)
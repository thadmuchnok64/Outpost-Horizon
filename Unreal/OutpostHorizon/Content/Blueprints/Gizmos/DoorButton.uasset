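; DoorButton is a gizmo that triggers a door from a physical button, but only once it has power.
; Tick polls the child Button actor and calls OnPicked on the Door when pressed while powered.
; A DoOnce limits this to one call per press, resetting whenever the button is released or power is off.
; The Power function sets the powered flag and swaps a CRTV material to show it.
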(event `self.ReceiveTick`
  (params (DeltaSeconds :type "Float (single-precision)"))
  (bind _asbutton (cast `/Game/Blueprints/Gizmos/Button` (`ChildActorComponent.ChildActor` (`self.Button`))))
  (if (`/Game/Blueprints/Gizmos/Button.IsBeingPressed` _asbutton)
    (if (`self.PowerOn`)
      (`/Engine/EditorBlueprintResources/StandardMacros.DoOnce` false :!label _label
        (:`Completed`
          (`/Game/Blueprints/Gizmos/Door.OnPicked` (`self.Door`))))
      (else
        (goto _label :!via `Reset`)))
    (else
      (goto _label :!via `Reset`))))

(fn `Power`
  (set `self.PowerOn` true)
  (`PrimitiveComponent.SetMaterial` (`self.CRTV`) 1 "/Game/Materials/CRTV/Power/PowerOn.PowerOn"))

(fn `UserConstructionScript`)
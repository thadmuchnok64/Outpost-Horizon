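; AdminDoorButton is a gizmo button with a CRTV screen that controls a door requiring admin access.
; It binds to DoorWay's unlock event, which sets an unlocked flag and swaps the screen to the unlocked material.
; Tick polls the child Button actor: a press while locked shows an access-needed screen and plays an error sound, while an unlocked press calls the door's OnPicked.
; Separate DoOnce gates without resets limit each response to once.
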(event `self.ReceiveBeginPlay`
  (add `/Game/Blueprints/BuildingBlocks/WallDoor.UnlockDoor` (`self.DoorWay`) (delegate `UnlockDoor`)))

(event `UnlockDoor`
  (set `self.Unlocked` true)
  (`PrimitiveComponent.SetMaterial` (`self.CRTV`) 1 "/Game/Materials/CRTV/Power/Unlocked.Unlocked"))

(event `self.ReceiveTick`
  (params (DeltaSeconds :type "Float (single-precision)"))
  (bind _crtv (`self.CRTV`))
  (bind _asbutton (cast `/Game/Blueprints/Gizmos/Button` (`ChildActorComponent.ChildActor` (`self.Button`))))
  (if (`/Game/Blueprints/Gizmos/Button.IsBeingPressed` _asbutton)
    (if (not (`self.Unlocked`))
      (`/Engine/EditorBlueprintResources/StandardMacros.DoOnce` false
        (:`Completed`
          (`PrimitiveComponent.SetMaterial` _crtv 1 "/Game/Materials/CRTV/Power/AdminAccessNeeded.AdminAccessNeeded")
          (`GameplayStatics.PlaySoundAtLocation` "/Game/Sounds/Sound_Effects/Error2.Error2" (`SceneComponent.K2_GetComponentLocation` _crtv) (struct) 1.0 1.0 0.0 null null null null)))
      (else
        (`/Engine/EditorBlueprintResources/StandardMacros.DoOnce` false
          (:`Completed`
            (`/Game/Blueprints/Gizmos/Door.OnPicked` (`self.Door`))))))))

(fn `UserConstructionScript`)
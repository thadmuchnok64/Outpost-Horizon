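; SillouetteSpook is a scare gizmo that plays a short animated silhouette when its Spook event is called.
; After a delay, it steps through frame textures on three planes like a flipbook, creating dynamic material instances at each step.
; From the second frame, the Scene component slides along X while the animation continues.
; The sequence ends by hiding AlarmBeam and playing a light flicker sound at its location.
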(event `Spook`
  (bind _delay (`self.Delay`))
  (bind _alarmbeam (`self.AlarmBeam`))
  (bind _array (`|MakeArray` (`self.Plane1`) (`self.Plane2`) (`self.Plane`)))
  (`KismetSystemLibrary.Delay` 1.0)
  (for _array_element _array
    (bind _returnvalue (`PrimitiveComponent.CreateDynamicMaterialInstance` _array_element 0 (`PrimitiveComponent.GetMaterial` _array_element 0) "None"))
    (`MaterialInstanceDynamic.SetTextureParameterValue` _returnvalue "Texture" "/Game/Materials/JJSpook/frame_1_delay-0_2s.frame_1_delay-0_2s"))
  (`KismetSystemLibrary.Delay` _delay)
  (for _array_element_2 _array
    (bind _returnvalue_2 (`PrimitiveComponent.CreateDynamicMaterialInstance` _array_element_2 0 (`PrimitiveComponent.GetMaterial` _array_element_2 0) "None"))
    (`MaterialInstanceDynamic.SetTextureParameterValue` _returnvalue_2 "Texture" "/Game/Materials/JJSpook/frame_2_delay-0_2s.frame_2_delay-0_2s"))
  (`|ExecutionSequence`
    (:`then_0`
      (`KismetSystemLibrary.Delay` (* _delay 1.0))
      (for _array_element_3 _array
        (bind _returnvalue_3 (`PrimitiveComponent.CreateDynamicMaterialInstance` _array_element_3 0 (`PrimitiveComponent.GetMaterial` _array_element_3 0) "None"))
        (`MaterialInstanceDynamic.SetTextureParameterValue` _returnvalue_3 "Texture" "/Game/Materials/JJSpook/frame_3_delay-0_2s.frame_3_delay-0_2s"))
      (`KismetSystemLibrary.Delay` _delay)
      (for _array_element_4 _array
        (bind _returnvalue_4 (`PrimitiveComponent.CreateDynamicMaterialInstance` _array_element_4 0 (`PrimitiveComponent.GetMaterial` _array_element_4 0) "None"))
        (`MaterialInstanceDynamic.SetTextureParameterValue` _returnvalue_4 "Texture" "/Game/Materials/JJSpook/frame_4_delay-0_2s.frame_4_delay-0_2s"))
      (`KismetSystemLibrary.Delay` _delay)
      (for _array_element_5 _array
        (bind _returnvalue_5 (`PrimitiveComponent.CreateDynamicMaterialInstance` _array_element_5 0 (`PrimitiveComponent.GetMaterial` _array_element_5 0) "None"))
        (`MaterialInstanceDynamic.SetTextureParameterValue` _returnvalue_5 "Texture" "/Game/Materials/JJSpook/frame_4_delay-0_2s.frame_4_delay-0_2s"))
      (`KismetSystemLibrary.Delay` 0.5)
      (`SceneComponent.SetVisibility` _alarmbeam false false)
      (`GameplayStatics.PlaySoundAtLocation` "/Game/Sounds/Sound_Effects/LightFlicker/LightFlicker.LightFlicker" (`SceneComponent.K2_GetComponentLocation` _alarmbeam) (struct) 1.0 1.0 0.0 "/Game/Sounds/Sound_Effects/Attenuation/MajorGizmo.MajorGizmo" null null null))
    (:`then_1`
      (`KismetSystemLibrary.MoveComponentTo` (`self.Scene`) (120.0 0.0 0.0) (struct) false true 0.4))))

(fn `UserConstructionScript`)
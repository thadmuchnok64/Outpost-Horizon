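; VR push button gizmo that sets IsBeingPressed based on how far its Press component moves from the root.
; Each Tick compares that distance to PressZone, with two cross-reset DoOnce gates firing press and release once per threshold crossing.
; Both transitions play a sound.
; Pressing also sends a haptic pulse to the hand of whichever VRPawn motion controller is closer to the button.
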(event `self.ReceiveActorBeginOverlap`
  (params (OtherActor :type "Actor Object Reference")))

(event `self.ReceiveTick`
  (params (DeltaSeconds :type "Float (single-precision)"))
  (bind _returnvalue (`self.K2_GetActorLocation`))
  (bind _presszone (`self.PressZone`))
  (if (>= (`KismetMathLibrary.FClamp` (`KismetMathLibrary.Vector_Distance` (`SceneComponent.K2_GetComponentLocation` (`self.DefaultSceneRoot`)) (`SceneComponent.K2_GetComponentLocation` (`self.Press`))) 0.0 (* _presszone 2.0)) _presszone)
    (`|ExecutionSequence`
      (:`then_0`
        (`/Engine/EditorBlueprintResources/StandardMacros.DoOnce` true :!label _label
          (:`Completed`
            (`GameplayStatics.PlaySoundAtLocation` "/Game/Sounds/Sound_Effects/Button_Press.Button_Press" _returnvalue (struct) 1.0 1.0 0.0 null null null null)
            (set `self.IsBeingPressed` true)
            (bind _outactors (`GameplayStatics.GetAllActorsOfClass` "/Game/VRTemplate/Blueprints/VRPawn.VRPawn_C"))
            (bind _returnvalue_2 (`self.K2_GetComponentsByClass` (`|GetArrayItem` _outactors) "/Script/HeadMountedDisplay.MotionControllerComponent"))
            (bind _output (`|GetArrayItem` _returnvalue_2 1))
            (bind _output_2 (`|GetArrayItem` _returnvalue_2))
            (`PlayerController.PlayHapticEffect` (`GameplayStatics.GetPlayerController` 0) "/Game/VRTemplate/Haptics/GrabHapticEffect.GrabHapticEffect" (select `bool` (< (`KismetMathLibrary.Vector_Distance` (`SceneComponent.K2_GetComponentLocation` (`self.Press`)) (`SceneComponent.K2_GetComponentLocation` _output_2)) (`KismetMathLibrary.Vector_Distance` (`SceneComponent.K2_GetComponentLocation` (`self.Press`)) (`SceneComponent.K2_GetComponentLocation` _output))) :`false` (select `bool` (== (`MotionControllerComponent.MotionSource` _output) "LeftGrip") :`false` "Right" :`true` "Left" :!type "EControllerHand Enum") :`true` (select `bool` (== (`MotionControllerComponent.MotionSource` _output_2) "LeftGrip") :`false` "Right" :`true` "Left" :!type "EControllerHand Enum")) 0.5 false))))
      (:`then_1`
        (goto _label_2 :!via `Reset`)))
    (else
      (`|ExecutionSequence`
        (:`then_0`
          (`/Engine/EditorBlueprintResources/StandardMacros.DoOnce` true :!label _label_2
            (:`Completed`
              (`GameplayStatics.PlaySoundAtLocation` "/Game/Sounds/Sound_Effects/Button_Release.Button_Release" _returnvalue (struct) 1.0 1.0 0.0 null null null null)
              (set `self.IsBeingPressed` false))))
        (:`then_1`
          (goto _label :!via `Reset`))))))

(fn `UserConstructionScript`)
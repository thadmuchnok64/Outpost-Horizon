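; Switch gizmo Blueprint that plays on and off sounds as its lever is flipped.
; BeginPlay assigns Pivot as the custom pivot of FlipLever.
; Tick polls FlipLever's SwitchState, using two DoOnce nodes that reset each other so each sound plays once per state change at the LeverPivot location.
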(event `self.ReceiveBeginPlay`
  (set `/Game/Blueprints/GrabbingStuff/GrabComponent.CustomPivot` (`self.Pivot`) (`self.FlipLever`)))

(event `self.ReceiveTick`
  (params (DeltaSeconds :type "Float (single-precision)"))
  (bind _returnvalue (`SceneComponent.K2_GetComponentLocation` (`self.LeverPivot`)))
  (if (`/Game/Blueprints/GrabbingStuff/GrabComponent.SwitchState` (`self.FlipLever`))
    (`|ExecutionSequence`
      (:`then_0`
        (`/Engine/EditorBlueprintResources/StandardMacros.DoOnce` false :!label _label
          (:`Completed`
            (`GameplayStatics.PlaySoundAtLocation` "/Game/Sounds/Sound_Effects/Switch_ON.Switch_ON" _returnvalue (struct) 1.0 1.0 0.0 null null null null))))
      (:`then_1`
        (goto _label_2 :!via `Reset`)))
    (else
      (`|ExecutionSequence`
        (:`then_0`
          (`/Engine/EditorBlueprintResources/StandardMacros.DoOnce` true :!label _label_2
            (:`Completed`
              (`GameplayStatics.PlaySoundAtLocation` "/Game/Sounds/Sound_Effects/Switch_OFF.Switch_OFF" _returnvalue (struct) 1.0 1.0 0.0 null null null null))))
        (:`then_1`
          (goto _label :!via `Reset`))))))

(fn `UserConstructionScript`)
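; Newspaper spook gizmo that makes a newspaper animation fly in when its Spooker fires.
; Once spooked, Tick accumulates time and scrubs NewspaperAnimV2 through its start time offset, using a clamped linear ramp instead of normal playback.
; When the ramp passes a set point, a DoOnce plays a heavy wet impact sound in 2D while the animation continues.
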(event `self.ReceiveBeginPlay`
  (add `/Game/Blueprints/Gizmos/ScareTrigger.Spook` (`self.Spooker`) (delegate `FlyIn`)))

(event `FlyIn`
  (set `self.Spooked` true))

(event `self.ReceiveTick`
  (params (DeltaSeconds :type "Float (single-precision)"))
  (if (`self.Spooked`)
    (bind _output_get (set `self.Timer` (+ DeltaSeconds (`self.Timer`))))
    (bind _returnvalue (`KismetMathLibrary.Lerp` 0.0 6.0 (/ _output_get 8.0)))
    (if (> _returnvalue 1.4)
      (`|ExecutionSequence`
        (:`then_0`
          (`GeometryCacheComponent.SetStartTimeOffset` (`self.Newspaper_Anim_V2`) (`KismetMathLibrary.FClamp` _returnvalue 0.0 6.0) :!label _label))
        (:`then_1`
          (`/Engine/EditorBlueprintResources/StandardMacros.DoOnce` false
            (:`Completed`
              (`GameplayStatics.PlaySound2D` "/Game/Sounds/Sound_Effects/Heavy__wet_impact.Heavy__wet_impact" 1.0 1.0 0.0 null null)))))
      (else
        (goto _label)))))

(fn `UserConstructionScript`)
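; Manager for the incinerator room that wraps the VR player's position and stages a hallucination scene.
; Four wall triggers teleport the VRPawn by a fixed offset toward the opposite side, looping the space.
; BeginPlay hides "Hallucination" actors; entering the room flickers spotlights off once, then hides "Disappearing" actors and reveals the hallucinations.
; An out-of-bounds player reset is present but unwired.
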(event `RightToLeft` :!signature `self.OnActorBeginOverlap`
  (params (OverlappedActor :type "Actor Object Reference") (OtherActor :type "Actor Object Reference"))
  ;[1 1 1] When player enters border, shift position to opposite side of inner square
  (set `self.TransformShift` (-1600.0 0.0 0.0))
  ;[1 1 1] Teleport Player
  (bind _outactors (`GameplayStatics.GetAllActorsOfClass` "/Game/VRTemplate/Blueprints/VRPawn.VRPawn_C" :!label _label))
  (for _array_element _outactors
    (`/Engine/EditorBlueprintResources/StandardMacros.DoOnce` false :!label _label_2
      (:`Completed`
        (bind _returnvalue_location (`KismetMathLibrary.BreakTransform` (`self.GetTransform` _array_element)))
        (`self.K2_SetActorLocationAndRotation` :`self` _array_element :`NewLocation` (+ _returnvalue_location (`self.TransformShift`)) :`bTeleport` true))))
  (goto _label_2 :!via `Reset`))

(event `LeftToRight` :!signature `self.OnActorBeginOverlap`
  (params (OverlappedActor :type "Actor Object Reference") (OtherActor :type "Actor Object Reference"))
  ;[1 1 1] When player enters border, shift position to opposite side of inner square
  (set `self.TransformShift` (1600.0 0.0 0.0))
  (goto _label))

(event `FrontToBack` :!signature `self.OnActorBeginOverlap`
  (params (OverlappedActor :type "Actor Object Reference") (OtherActor :type "Actor Object Reference"))
  ;[1 1 1] When player enters border, shift position to opposite side of inner square
  (set `self.TransformShift` (0.0 -1600.0 0.0))
  (goto _label))

(event `BackToFront` :!signature `self.OnActorBeginOverlap`
  (params (OverlappedActor :type "Actor Object Reference") (OtherActor :type "Actor Object Reference"))
  ;[1 1 1] When player enters border, shift position to opposite side of inner square
  (set `self.TransformShift` (0.0 1600.0 0.0))
  (goto _label))

(event `self.ReceiveBeginPlay`
  (bind _outactors (`GameplayStatics.GetAllActorsWithTag` "Hallucination"))
  (for _array_element _outactors
    (`self.SetActorHiddenInGame` _array_element true))
  ;[1 1 1] When player enters scene, start Lights Flicker event
  (add `self.OnActorBeginOverlap` (`self.Enter Trigger Volume`) (delegate `OnActorBeginOverlap_Event_0`))
  ;[1 1 1] When player enters border, shift position to opposite side of inner square
  (add `self.OnActorBeginOverlap` (`self.BackWall`) (delegate `BackToFront`))
  (add `self.OnActorBeginOverlap` (`self.FrontWall`) (delegate `FrontToBack`))
  (add `self.OnActorBeginOverlap` (`self.LeftWall`) (delegate `LeftToRight`))
  (add `self.OnActorBeginOverlap` (`self.RightWall`) (delegate `RightToLeft`)))

(event `OnActorBeginOverlap_Event`
  (params (OverlappedActor :type "Actor Object Reference") (OtherActor :type "Actor Object Reference"))
  ;[1 1 1] When player enters border, shift position to opposite side of inner square
)

(event `ResetPlayerPosition`
  ;[1 1 1] Reset Player Location
)

(event `OnActorBeginOverlap_Event_0` :!signature `self.OnActorBeginOverlap`
  (params (OverlappedActor :type "Actor Object Reference") (OtherActor :type "Actor Object Reference"))
  ;[1 1 1] When player enters scene, start Lights Flicker event
  (for _array_element (`self.GetOverlappingActors` (`self.Enter Trigger Volume`) null)
    (cast `/Game/VRTemplate/Blueprints/VRPawn` _array_element)
    (`/Engine/EditorBlueprintResources/StandardMacros.DoOnce` false
      (:`Completed`
        (`self.FlickerLights`)))))

(event `FlickerLights`
  ;[1 1 1] Flicker Lights
  (for _array_element (`self.Flickering Lights`)
    (bind _asspot_light (cast `SpotLight` _array_element))
    (bind _lightcomponent (`Light.LightComponent` _asspot_light))
    (`SceneComponent.SetVisibility` _lightcomponent false false)
    (`KismetSystemLibrary.Delay` 0.5)
    (`SceneComponent.SetVisibility` _lightcomponent true false)
    (`KismetSystemLibrary.Delay` 1.0)
    (`SceneComponent.SetVisibility` _lightcomponent false false)
    (`KismetSystemLibrary.Delay` 0.3)
    (`SceneComponent.SetVisibility` _lightcomponent true false)
    (`KismetSystemLibrary.Delay` 0.5)
    (`SceneComponent.SetVisibility` _lightcomponent false false)
    (`KismetSystemLibrary.Delay` 0.2)
    (`SceneComponent.SetVisibility` _lightcomponent true false)
    (`KismetSystemLibrary.Delay` 0.3)
    (`SceneComponent.SetVisibility` _lightcomponent false false)
    (bind _outactors (`GameplayStatics.GetAllActorsWithTag` "Disappearing"))
    (for _array_element_2 _outactors
      (`self.SetActorHiddenInGame` _array_element_2 true)
      (bind _outactors_2 (`GameplayStatics.GetAllActorsWithTag` "Hallucination"))
      (for _array_element_3 _outactors_2
        (`self.SetActorHiddenInGame` _array_element_3 false)))))

(fn `UserConstructionScript`)
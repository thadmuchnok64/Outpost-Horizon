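; Office room shutters that play an activation sound and trigger the TitleMesh logo when CallShutters first fires.
; Tick then scrubs five shutter components by lerping their start time offsets over an accumulated timer, stopping at about twice LerpTime.
; ShuttersMidLeft fakes a broken shutter: a second timer subtracted from the main one makes it nearly stall partway, then rapidly speed up.
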(event `CallShutters`
  (if (not (`self.ShuttersActivated`))
    (`GameplayStatics.PlaySoundAtLocation` "/Game/Sounds/Sound_Effects/ShuttersActivate.ShuttersActivate" (`self.K2_GetActorLocation`) (struct) 1.0 1.0 0.0 "/Game/Sounds/Sound_Effects/Attenuation/SmallGizmo.SmallGizmo" null null null)
    (set `self.ShuttersActivated` true)
    (bind _returnvalue (`GameplayStatics.GetActorOfClass` "/Game/TitleMesh.TitleMesh_C"))
    (`/Game/TitleMesh.Call Logo` _returnvalue)))

(event `self.ReceiveTick`
  (params (DeltaSeconds :type "Float (single-precision)"))
  (bind _returnvalue (+ DeltaSeconds (`self.Timer`)))
  (bind _returnvalue_2 (/ (`self.Timer`) (`self.LerpTime`)))
  (bind _returnvalue_3 (`KismetMathLibrary.Lerp` 0.0 6.0 _returnvalue_2))
  (if (`self.ShuttersActivated`)
    (set `self.Timer` _returnvalue)
    (set `self.BrokenTimer` (+ (`self.BrokenTimer`) (* DeltaSeconds 0.95)))
    (if (not (> (/ _returnvalue (`self.LerpTime`)) 2.0))
      (`|ExecutionSequence`
        (:`then_0`
          (for _array_element (`|MakeArray` (`self.Shutters_Left`) (`self.Shutters_Right`) (`self.Shutters_Mid_Right`) (`self.Shutters_Mid`))
            (`GeometryCacheComponent.SetStartTimeOffset` _array_element _returnvalue_3)))
        (:`then_1`
          (if (> _returnvalue_2 0.45)
            (if (> _returnvalue_2 0.8)
              (set `self.BrokenTimer` (- (`self.BrokenTimer`) (* DeltaSeconds 10.0))))
            (`GeometryCacheComponent.SetStartTimeOffset` (`self.Shutters_Mid_Left`) (`KismetMathLibrary.Lerp` 0.0 6.0 (/ (- (`self.Timer`) (`self.BrokenTimer`)) (`self.LerpTime`))))
            (else
              (set `self.BrokenTimer` 0.0)
              (`GeometryCacheComponent.SetStartTimeOffset` (`self.Shutters_Mid_Left`) _returnvalue_3))))))))

(fn `UserConstructionScript`)
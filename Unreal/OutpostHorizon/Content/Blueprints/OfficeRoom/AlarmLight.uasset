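; Office room alarm light that switches to a red, spinning beacon when its alarm is triggered.
; BeginPlay sets the LED material on the light mesh and hides the beam.
; AlarmActivate shows the beam, swaps in the red material and sets a flag that lets Tick rotate the beam about its roll axis from accumulated time.
; The file has no event to switch the alarm off.
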(event `self.ReceiveBeginPlay`
  (`PrimitiveComponent.SetMaterial` (`self.Lights`) 1 "/Game/Meshes/EnviormentalAssets/Light/LED.LED")
  (`SceneComponent.SetVisibility` (`self.AlarmBeam`) false false))

(event `AlarmActivate`
  (set `self.AlarmActive` true)
  (`SceneComponent.SetVisibility` (`self.AlarmBeam`) true false)
  (`PrimitiveComponent.SetMaterial` (`self.Lights`) 1 "/Game/Meshes/EnviormentalAssets/Light/LightRed.LightRed"))

(event `self.ReceiveTick`
  (params (DeltaSeconds :type "Float (single-precision)"))
  (if (`self.AlarmActive`)
    (bind _output_get (set `self.Timer` (+ DeltaSeconds (`self.Timer`))))
    (`SceneComponent.K2_SetRelativeRotation` (`self.AlarmBeam`) (`KismetMathLibrary.MakeRotator` (* _output_get 180.0) 0.0 -90.0) false false)))

(fn `UserConstructionScript`)
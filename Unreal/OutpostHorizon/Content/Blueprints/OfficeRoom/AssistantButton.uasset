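; Office assistant console with CRT screens, radio audio and a glass-covered button that opens the elevator door and calls the shutters.
; BeginPlay freezes the child-actor button, plays radio static and starts an intro video on one screen.
; AssistantOnline flickers the other screens to online visuals, switches audio, animates the glass and unfreezes the blinking button; AssistantOffline swaps one screen to off.
; Tick polls the button, using DoOnce to fire once per press.
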(event `self.ReceiveBeginPlay`
  (bind _audio (`self.Audio`))
  (bind _asbutton (cast `/Game/Blueprints/Gizmos/Button` (`ChildActorComponent.ChildActor` (`self.Button`))))
  (`/Game/Blueprints/Gizmos/Button.FreezeButton` _asbutton true)
  (`AudioComponent.SetSound` _audio "/Game/Sounds/Sound_Effects/RadioStatic.RadioStatic")
  (`AudioComponent.Play` _audio 0.0)
  (`KismetSystemLibrary.Delay` 2.0)
  (`PrimitiveComponent.SetMaterial` (`self.CRTV2`) 1 "/Game/Videos/TestVideoMat.TestVideoMat")
  (`MediaPlayer.OpenSource` (`self.media`) "/Game/Videos/IntroVideo.IntroVideo"))

(event `self.ReceiveTick`
  (params (DeltaSeconds :type "Float (single-precision)"))
  (bind _asbutton (cast `/Game/Blueprints/Gizmos/Button` (`ChildActorComponent.ChildActor` (`self.Button`))))
  (if (`/Game/Blueprints/Gizmos/Button.IsBeingPressed` _asbutton)
    (`/Engine/EditorBlueprintResources/StandardMacros.DoOnce` false :!label _label
      (:`Completed`
        (set `/Game/Blueprints/Gizmos/ElevatorPort.DoorOpen` true (`self.ElevatorPort`))
        (`/Game/Blueprints/OfficeRoom/Shutters.CallShutters` (`self.Shutters`))))
    (else
      (goto _label :!via `Reset`))))

(event `SetOnline`
  (bind _audio (`self.Audio`))
  (`PrimitiveComponent.SetMaterial` (`self.CRTV`) 1 "/Game/Materials/CRTV/Power/Static.Static")
  (`KismetSystemLibrary.Delay` 0.2)
  (`PrimitiveComponent.SetMaterial` (`self.CRTV1`) 1 "/Game/Materials/CRTV/Power/Static.Static")
  (`KismetSystemLibrary.Delay` 0.5)
  (`PrimitiveComponent.SetMaterial` (`self.CRTV`) 1 "/Game/Materials/CRTV/Power/AssistantOnline.AssistantOnline")
  (`KismetSystemLibrary.Delay` 0.2)
  (`PrimitiveComponent.SetMaterial` (`self.CRTV1`) 1 "/Game/Materials/CRTV/Power/Start.Start")
  (`AudioComponent.Stop` _audio)
  (`AudioComponent.SetSound` _audio "/Game/Sounds/Sound_Effects/RadioConnection.RadioConnection")
  (`AudioComponent.Play` _audio 0.0)
  (`SkeletalMeshComponent.PlayAnimation` (`self.Button_Glass`) "/Game/Meshes/Gizmos/Button/Button_Glass_Anim.Button_Glass_Anim" false)
  (bind _asbutton (cast `/Game/Blueprints/Gizmos/Button` (`ChildActorComponent.ChildActor` (`self.Button`))))
  (`PrimitiveComponent.SetMaterial` (`/Game/Blueprints/Gizmos/Button.Press` _asbutton) 0 "/Game/Materials/Button/BlinkyButton.BlinkyButton")
  (`/Game/Blueprints/Gizmos/Button.FreezeButton` _asbutton false))

(fn `AssistantOffline`
  (`PrimitiveComponent.SetMaterial` (`self.CRTV`) 1 "/Game/Materials/CRTV/Power/AssistantOff.AssistantOff"))

(fn `AssistantOnline`
  (`self.SetOnline`))

(fn `UserConstructionScript`)
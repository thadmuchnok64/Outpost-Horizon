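; Fuel rod slot actor in the engine room that holds one fuel rod, starting with the rod from its child actor.
; Inserting and removing swap the stored reference with a sound, removal also activating a dust effect, and breaking is forwarded to the rod.
; The working check requires a valid, working rod whose substance matches the desired type, except Unobtainium, which skips the type match.
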(event `self.ReceiveBeginPlay`
  (bind _asfuel_rod_blueprint (cast `/Game/Blueprints/EngineRoom/Fuel_Rod_Blueprint` (`ChildActorComponent.ChildActor` (`self.Fuel_Rod_Blueprint`))))
  (set `self.rod` _asfuel_rod_blueprint))

(fn `BreakRod`
  (`/Game/Blueprints/EngineRoom/Fuel_Rod_Blueprint.BreakRod` (`self.rod`)))

(fn `InsertRod`
  (params (Rod :type "Actor Object Reference"))
  (bind _asfuel_rod_blueprint (cast `/Game/Blueprints/EngineRoom/Fuel_Rod_Blueprint` Rod))
  (`GameplayStatics.PlaySound2D` "/Game/Sounds/Sound_Effects/Insert.Insert" 1.0 1.0 0.0 null null)
  (set `self.rod` _asfuel_rod_blueprint))

(fn `Is Rod Working`
  (returns (RodIsWorking :type Boolean))
  (bind _rod (`self.rod`))
  (bind _substancetype (`/Game/Blueprints/EngineRoom/Fuel_Rod_Blueprint.SubstanceType` _rod))
  (if (`KismetSystemLibrary.IsValid` _rod)
    (switch `/Game/Blueprints/EngineRoom/FuelRodType` _substancetype
      (:`NewEnumerator0`
        (if (== (`KismetMathLibrary.Conv_ByteToInt` _substancetype) (`KismetMathLibrary.Conv_ByteToInt` (`self.DesiredRod`))) :!label _label
          _
          (else
            (return false))))
      (:`NewEnumerator1`
        (goto _label))
      (:`NewEnumerator2`
        (goto _label))
      (:`NewEnumerator3`
        (goto _label))
      (:`NewEnumerator4`
        (goto _label))
      (:`NewEnumerator5`
        _))
    (return (`/Game/Blueprints/EngineRoom/Fuel_Rod_Blueprint.IsWorking` _rod))
    (else
      (return false))))

(fn `RemoveRod`
  (`GameplayStatics.PlaySound2D` "/Game/Sounds/Sound_Effects/Eject.Eject" 1.0 1.0 0.0 null null)
  (`ActorComponent.Activate` (`self.Dust_System`) false)
  (set `self.rod` null))

(fn `UserConstructionScript`)
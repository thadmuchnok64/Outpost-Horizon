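; Engine actor for the engine room, managing seven fuel rod slots and reporting broken rods to a server.
; Two seconds after BeginPlay it caches the slots, then breaks randomly chosen rods via a shuffled array copy.
; That breakdown, or flipping the child switch on (polled on Tick), sends broken slot numbers through the tagged TCPClient.
; A start sound plays when none are broken.
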(event `self.ReceiveBeginPlay`
  (`|ExecutionSequence`
    (:`then_0`
      ;[0.6979 1 0.7664] Assign Slot Variables
      (bind _asfuel_rod_slot (cast `/Game/Blueprints/EngineRoom/Fuel_Rod_Slot` (`ChildActorComponent.ChildActor` (`self.Fuel_Rod_Slot4`)))))
    (:`then_1`
      (bind _asfuel_rod_slot_2 (cast `/Game/Blueprints/EngineRoom/Fuel_Rod_Slot` (`ChildActorComponent.ChildActor` (`self.Fuel_Rod_Slot6`)))))
    (:`then_2`
      (bind _asfuel_rod_slot_3 (cast `/Game/Blueprints/EngineRoom/Fuel_Rod_Slot` (`ChildActorComponent.ChildActor` (`self.Fuel_Rod_Slot1`)))))
    (:`then_3`
      (bind _asfuel_rod_slot_4 (cast `/Game/Blueprints/EngineRoom/Fuel_Rod_Slot` (`ChildActorComponent.ChildActor` (`self.Fuel_Rod_Slot3`)))))
    (:`then_4`
      (bind _asfuel_rod_slot_5 (cast `/Game/Blueprints/EngineRoom/Fuel_Rod_Slot` (`ChildActorComponent.ChildActor` (`self.Fuel_Rod_Slot2`)))))
    (:`then_5`
      (bind _asfuel_rod_slot_6 (cast `/Game/Blueprints/EngineRoom/Fuel_Rod_Slot` (`ChildActorComponent.ChildActor` (`self.Fuel_Rod_Slot`)))))
    (:`then_6`
      (bind _asfuel_rod_slot_7 (cast `/Game/Blueprints/EngineRoom/Fuel_Rod_Slot` (`ChildActorComponent.ChildActor` (`self.Fuel_Rod_Slot5`))))
      (set `self.FuelRodSlots` (`|MakeArray` _asfuel_rod_slot _asfuel_rod_slot_2 _asfuel_rod_slot_3 _asfuel_rod_slot_4 _asfuel_rod_slot_5 _asfuel_rod_slot_6 _asfuel_rod_slot_7)))
    (:`then_7`
      (`KismetSystemLibrary.Delay` 2.0)
      (`self.Breakdown`))))

(event `self.ReceiveTick`
  (params (DeltaSeconds :type "Float (single-precision)"))
  ;[1 0.1143 0.1342] Checks if switch is flipped
  (bind _asswitch_blueprint (cast `/Game/Switch_Blueprint` (`ChildActorComponent.ChildActor` (`self.Switch_Blueprint`))))
  (bind _switchstate (`/Game/VRTemplate/Blueprints/GrabComponent.SwitchState` (`/Game/Switch_Blueprint.Grab` _asswitch_blueprint)))
  (if (!= _switchstate (`self.Switch`))
    (bind _output_get (set `self.Switch` _switchstate))
    (if _output_get
      ;[0.6832 1 0.7694] Construct message from broken rods
      (bind _output_get_2 (set `self.RodMessage` (`|MakeArray`) :!label _label))
      (for (_array_element _array_index) (`self.FuelRodSlots`)
        (bind _rodisworking (`/Game/Blueprints/EngineRoom/Fuel_Rod_Slot.Is Rod Working` _array_element))
        (if (not _rodisworking)
          (`KismetArrayLibrary.Array_Append` _output_get_2 (`|MakeArray` (+ _array_index 1)))))
      (if (<= (`KismetArrayLibrary.Array_Length` _output_get_2) 0)
        (`GameplayStatics.PlaySound2D` "/Game/Sounds/Sound_Effects/CarStart.CarStart" 1.0 1.0 0.0 null null))
      ;[0.06383 0.3331 1] Send message to server
      (bind _outactors (`GameplayStatics.GetAllActorsWithTag` "TCP"))
      (bind _astcpclient (cast `/Game/NetworkStuff/TCPClient` (`|GetArrayItem` _outactors))
        (:`then`
          (`/Game/NetworkStuff/TCPClient.SendIntegersToServer` _astcpclient 3 (`self.RodMessage`)))
        (:`CastFailed`
          (`KismetSystemLibrary.PrintString` "no work"))))))

(event `Breakdown`
  (bind _temparray (`self.TempArray`))
  ;[0.08404 0.7374 1] Break Rods
  (bind _output_get (set `self.TempArray` (`|MakeArray` null :!type "/Game/Blueprints/EngineRoom/Fuel_Rod_Slot Object Reference")))
  (`KismetArrayLibrary.Array_Append` _output_get (`self.FuelRodSlots`))
  (`KismetArrayLibrary.Array_Shuffle` _temparray)
  (for _index (range (+ 2 1))
    (`/Game/Blueprints/EngineRoom/Fuel_Rod_Slot.BreakRod` (`|GetArrayItem` _temparray _index)))
  (goto _label))

(fn `UserConstructionScript`)
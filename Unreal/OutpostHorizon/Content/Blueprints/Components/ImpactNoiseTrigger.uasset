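; ImpactNoiseTrigger plays an attenuated impact sound when an impulse is strong enough.
; SoundManagement takes an impulse and origin, and above a magnitude threshold primes MetalClinks, then plays SoundCollection at that origin with SmallGizmo attenuation.
; The event graph is inactive, holding only a disconnected draft of the same logic that plays at GrabComponent's location.
; Nothing in this file calls SoundManagement.
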(fn `SoundManagement`
  (params (Impulse :type "Vector Structure") (SoundOrigin :type "Vector Structure"))
  (if (> (`KismetMathLibrary.VSize` Impulse) 700.0)
    (`AudioMixerBlueprintLibrary.PrimeSoundCueForPlayback` "/Game/Sounds/Sound_Effects/MetalImpact/MetalClinks.MetalClinks")
    (`GameplayStatics.PlaySoundAtLocation` (`self.SoundCollection`) SoundOrigin (struct) 0.8 1.0 0.0 "/Game/Sounds/Sound_Effects/Attenuation/SmallGizmo.SmallGizmo" null null null)))
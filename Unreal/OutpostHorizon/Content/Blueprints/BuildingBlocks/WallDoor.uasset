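; WallDoor is a building-block door that can be unlocked remotely through the TCPClient actor.
; On BeginPlay it binds to the client's remote-open and admin-grant events, acting on a matching door code.
; An Admin-flagged door sends function code 14 to the server; a grant clears the flag and resumes unlocking.
; Unlocking calls UnlockDoor and reports success to the server, while the local Unlock function only calls UnlockDoor.
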(event `self.ReceiveBeginPlay`
  (bind _returnvalue (`GameplayStatics.GetActorOfClass` "/Game/NetworkStuff/TCPClient.TCPClient_C"))
  (add `/Game/NetworkStuff/TCPClient.OpenDoorRemotely` _returnvalue (delegate `UnlockTime`))
  (add `/Game/NetworkStuff/TCPClient.GrantAdminAccess` _returnvalue (delegate `GrantAdmin`)))

(event `UnlockTime`
  (params (DoorCode :type Integer))
  (if (== DoorCode (`self.DoorCode`))
    (if (`self.Admin`) :!label _label
      (bind _returnvalue (`GameplayStatics.GetActorOfClass` "/Game/NetworkStuff/TCPClient.TCPClient_C"))
      (`/Game/NetworkStuff/TCPClient.SendIntegersToServer` _returnvalue 14 (`|MakeArray` (`self.DoorCode`)))
      (else
        (`self.UnlockDoor`)
        (bind _returnvalue_2 (`GameplayStatics.GetActorOfClass` "/Game/NetworkStuff/TCPClient.TCPClient_C"))
        (`/Game/NetworkStuff/TCPClient.Send Door Unlock Success` _returnvalue_2 (`self.DoorCode`))))))

(event `GrantAdmin`
  (params (`Door Code` :type Integer))
  (if (== `Door Code` (`self.DoorCode`))
    (set `self.Admin` false)
    (goto _label)))

(fn `Unlock`
  (`self.UnlockDoor`))

(fn `UserConstructionScript`)
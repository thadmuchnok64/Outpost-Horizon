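; Incinerator room actor that rearranges itself when a VR pawn enters its overlap area, apparently expanding the space.
; BeginPlay hides a set of incinerator floor pieces and the surrounding ceilings, which the overlap makes visible again.
; The overlap then launches parallel eased MoveComponentTo calls on the floor, wall, door and ceiling groups toward fixed relative locations, all timed by TimeToLerp.
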(event `self.ReceiveBeginPlay`
  (for _array_element (`|MakeArray` (`self.Incinerator_Floor5`) (`self.Incinerator_Floor1`) (`self.Incinerator_Floor4`) (`self.Incinerator_Floor3`) (`self.Incinerator_Floor2`) (`self.Incinerator_Floor8`))
    (`SceneComponent.SetVisibility` _array_element false true)
    (`SceneComponent.SetVisibility` (`self.SurroundingCeilings`) false true)))

(event `self.ReceiveActorBeginOverlap`
  (params (OtherActor :type "Actor Object Reference"))
  (bind _timetolerp (`self.TimeToLerp`))
  (cast `/Game/VRTemplate/Blueprints/VRPawn` OtherActor)
  (`SceneComponent.SetVisibility` (`self.SurroundingCeilings`) true true)
  (for _array_element (`|MakeArray` (`self.Incinerator_Floor5`) (`self.Incinerator_Floor1`) (`self.Incinerator_Floor4`) (`self.Incinerator_Floor3`) (`self.Incinerator_Floor2`) (`self.Incinerator_Floor8`))
    (`SceneComponent.SetVisibility` _array_element true false))
  (`|ExecutionSequence`
    (:`then_0`
      (`KismetSystemLibrary.MoveComponentTo` (`self.FloorGroup`) (0.0 -1440.0 0.0) (struct) true false _timetolerp))
    (:`then_1`
      (`KismetSystemLibrary.MoveComponentTo` (`self.Backwalls`) (0.0 -2880.0 0.0) (struct) true false _timetolerp))
    (:`then_2`
      (`KismetSystemLibrary.MoveComponentTo` (`self.WallDoorParent`) (0.0 0.0 -360.0) (struct) true false _timetolerp))
    (:`then_3`
      (`KismetSystemLibrary.MoveComponentTo` (`self.RightWalls`) (1440.0 -1440.0 0.0) (struct) true false _timetolerp))
    (:`then_4`
      (`KismetSystemLibrary.MoveComponentTo` (`self.LeftWalls`) (-1440.0 -1440.0 0.0) (struct) true false _timetolerp))
    (:`then_5`
      (`KismetSystemLibrary.MoveComponentTo` (`self.SurroundingCeilings`) (0.0 -1440.0 0.0) (struct) true false _timetolerp))
    (:`then_6`
      (`KismetSystemLibrary.MoveComponentTo` (`self.Ceiling`) (0.0 -1440.0 0.0) (struct) true false _timetolerp))))

(fn `UserConstructionScript`)
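; Crane control panel actor that lets the player drive the Crane_New found in the level.
; Each tick it reads two child-actor SlideLevers for forward/back and up/down movement, applying a deadzone.
; Only the forward/back axis sends zero inside the deadzone; up/down makes no call.
; A child Button calls TryAttach on the crane once per press, using a DoOnce that resets on release.
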(event `self.ReceiveBeginPlay`
  (bind _returnvalue (`GameplayStatics.GetActorOfClass` "/Game/Blueprints/CraneRoom/Crane_New.Crane_New_C"))
  (set `self.CraneNew` _returnvalue))

(event `self.ReceiveTick`
  (params (DeltaSeconds :type "Float (single-precision)"))
  (`|ExecutionSequence`
    (:`then_0`
      (bind _asslide_lever (cast `/Game/Blueprints/Gizmos/SlideLever` (`ChildActorComponent.ChildActor` (`self.BackwardForward_Lever`))))
      (bind _rawlevervalue (`/Game/VRTemplate/Blueprints/GrabComponent.RawLeverValue` (`/Game/Blueprints/Gizmos/SlideLever.GrabComponent` _asslide_lever)))
      (if (> (`KismetMathLibrary.Abs` _rawlevervalue) 0.1)
        (`/Game/Blueprints/CraneRoom/Crane_New.MoveFB` (`self.CraneNew`) _rawlevervalue)
        (else
          (`/Game/Blueprints/CraneRoom/Crane_New.MoveFB` (`self.CraneNew`) 0.0))))
    (:`then_1`
      (bind _asslide_lever_2 (cast `/Game/Blueprints/Gizmos/SlideLever` (`ChildActorComponent.ChildActor` (`self.UpDown_Lever`))))
      (bind _rawlevervalue_2 (`/Game/VRTemplate/Blueprints/GrabComponent.RawLeverValue` (`/Game/Blueprints/Gizmos/SlideLever.GrabComponent` _asslide_lever_2)))
      (if (> (`KismetMathLibrary.Abs` _rawlevervalue_2) 0.1)
        (`/Game/Blueprints/CraneRoom/Crane_New.MoveUD` (`self.CraneNew`) _rawlevervalue_2)))
    (:`then_2`
      (bind _asbutton (cast `/Game/Blueprints/Gizmos/Button` (`ChildActorComponent.ChildActor` (`self.Button`))))
      (if (`/Game/Blueprints/Gizmos/Button.IsBeingPressed` _asbutton)
        (`/Engine/EditorBlueprintResources/StandardMacros.DoOnce` false :!label _label
          (:`Completed`
            (`/Game/Blueprints/CraneRoom/Crane_New.TryAttach` (`self.CraneNew`))))
        (else
          (goto _label :!via `Reset`))))))

(fn `UserConstructionScript`)
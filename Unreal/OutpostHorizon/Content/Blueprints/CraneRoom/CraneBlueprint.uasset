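; Crane actor that moves its BackForth and UpDown components along X and Z in response to a signed magnitude.
; MoveForwardOrBack targets either horizontal limit, while MoveUpOrDown targets zero or the lowest point, each passing to an event that runs MoveComponentTo.
; Duration is the axis's max distance over speed times magnitude, regardless of current position.
; Zero magnitude issues no move or stop.
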(event `MoveForwardBackward`
  (params (Location :type "Vector Structure") (Duration :type "Float (double-precision)"))
  (`KismetSystemLibrary.MoveComponentTo` (`self.Back/Forth`) Location (struct) false false Duration))

(event `MoveUpDown`
  (params (Location :type "Vector Structure") (Duration :type "Float (double-precision)"))
  (`KismetSystemLibrary.MoveComponentTo` (`self.Up/Down`) Location (struct) false false Duration))

(fn `MoveForwardOrBack`
  (params (Magnitude :type "Float (double-precision)"))
  (if (!= Magnitude 0.0)
    (`self.MoveForwardBackward` (`KismetMathLibrary.MakeVector` (* (`KismetMathLibrary.SignOfFloat` Magnitude) (`self.MaxDistanceBackForth`))) (/ (`self.MaxDistanceBackForth`) (* (`KismetMathLibrary.Abs` Magnitude) (`self.HorizontalSpeed`))))))

(fn `MoveUpOrDown`
  (params (Magnitude :type "Float (double-precision)"))
  (if (!= Magnitude 0.0)
    (`self.MoveUpDown` (`KismetMathLibrary.MakeVector` 0.0 0.0 (`KismetMathLibrary.FClamp` (* (`KismetMathLibrary.SignOfFloat` Magnitude) (`self.MaxDistanceUpDown`)) (* (`self.MaxDistanceUpDown`) -1.0) 0.0)) (/ (`self.MaxDistanceUpDown`) (* (`KismetMathLibrary.Abs` Magnitude) (`self.VerticalSpeed`))))))

(fn `UserConstructionScript`)
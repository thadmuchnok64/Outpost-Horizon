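; Debug actor that lets the game be played without the mobile player, though rod order must be memorized.
; On BeginPlay, if EnableDebug is set, it puts the AssistantButton online and unlocks every DoorSteamButton.
; Every Tick, regardless of that flag, it writes a lock-pick message to the TCPClient.
; Tick also finds the Elevator nearest the VRPawn and moves it while its child button is pressed.
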(event `self.ReceiveBeginPlay`
  ;[1 1 1] Sets Doors to open and allows game to be played without mobile player. Rod order must be memorized.
  (if (`self.EnableDebug`)
    (bind _returnvalue (`GameplayStatics.GetActorOfClass` "/Game/Blueprints/OfficeRoom/AssistantButton.AssistantButton_C"))
    (`/Game/Blueprints/OfficeRoom/AssistantButton.SetOnline` _returnvalue)
    (bind _outactors (`GameplayStatics.GetAllActorsOfClass` "/Game/Blueprints/Gizmos/DoorSteamButton.DoorSteamButton_C"))
    (for _array_element _outactors
      (set `/Game/Blueprints/Gizmos/DoorSteamButton.Locked` false _array_element))))

(event `self.ReceiveTick`
  (params (DeltaSeconds :type "Float (single-precision)"))
  ;[1 1 1] Constantly picks door lock
  (bind _returnvalue (`GameplayStatics.GetActorOfClass` "/Game/NetworkStuff/TCPClient.TCPClient_C"))
  (set `/Game/NetworkStuff/TCPClient.TCPMessage` "PickTrue" _returnvalue)
  ;[1 1 1] Uses button to move elevator closest to player
  (bind _returnvalue_2 (`GameplayStatics.GetActorOfClass` "/Game/VRTemplate/Blueprints/VRPawn.VRPawn_C"))
  (bind _outactors (`GameplayStatics.GetAllActorsOfClass` "/Game/Blueprints/Gizmos/Elevator.Elevator_C"))
  (bind _aselevator (cast `/Game/Blueprints/Gizmos/Elevator` (`.ReturnValue` (`GameplayStatics.FindNearestActor` (`CharacterMovementComponent.GetLastUpdateLocation` (`Character.CharacterMovement` _returnvalue_2)) _outactors))))
  (bind _asbutton (cast `/Game/Blueprints/Gizmos/Button` (`ChildActorComponent.ChildActor` (`/Game/Blueprints/Gizmos/Elevator.Button` _aselevator))))
  (if (`/Game/Blueprints/Gizmos/Button.IsBeingPressed` _asbutton)
    (`/Game/Blueprints/Gizmos/Elevator.MoveElevator` _aselevator)))

(fn `UserConstructionScript`)